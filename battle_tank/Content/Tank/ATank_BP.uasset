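; Player-controlled tank Blueprint that wires up its weapon and movement components and maps input to tank actions.
; BeginPlay registers components and UI, gives StraightWeapon the turret, barrel and two projectile types with ammo, and hands both tracks to ForceNavMovement.
; Input events forward movement, aim lock, firing, burst, reload and projectile switching to functions defined outside these graphs.
; Look axes rotate Scene yaw and SpringArm pitch, scaled by delta time.
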(event EventBeginPlay
  (bind _straightweapon (Variables|Default|GetStraightWeapon))
  ;[1 1 1] Setup
  (Class|Tank|SetupComponent (Variables|Default|GetStraightWeapon) (Variables|Default|GetForceNavMovement))
  (Class|Tank|SetupUi)
  (Class|AimingComponent|Setup (Variables|Default|GetStraightWeapon) (Variables|Default|GetTankTurrent) (Variables|Default|GetTankBarrel))
  (Class|StraightWeaponComponent|AddProjectile _straightweapon "/Game/Projectile/a_projectile.a_projectile_C" 1)
  (Class|StraightWeaponComponent|AddProjectile _straightweapon "/Game/Projectile/b_projectile.b_projectile_C" 120)
  (Class|ForceNavMovementComponent|Setup (Variables|Default|GetForceNavMovement) (Variables|Default|Getleft_track) (Variables|Default|Getright_track)))

(event Input|ActionEvents|InputActionreload
  (params (Key :type Key%20Structure))
  ;[1 1 1] Weapon
  (:Pressed
    (Class|Tank|Reload)))

(event Input|ActionEvents|InputActionfire
  (params (Key :type Key%20Structure))
  ;[1 1 1] Weapon
  (:Pressed
    (Class|Tank|Fire)))

(event Input|ActionEvents|InputActionburst
  (params (Key :type Key%20Structure))
  ;[1 1 1] Move
  (:Pressed
    (Class|Tank|Burst true))
  (:Released
    (Class|Tank|Burst false)))

(event Input|ActionEvents|InputActionaiming
  (params (Key :type Key%20Structure))
  ;[1 1 1] Aiming
  (:Pressed
    (Class|Tank|Lock true))
  (:Released
    (Class|Tank|Lock false)))

(event Input|ActionEvents|InputActionexchange_weapon
  (params (Key :type Key%20Structure))
  ;[1 1 1] Weapon
  (:Pressed
    (Class|Tank|ExchangeProjectile)))

(event Input|ActionEvents|InputActionweapon_0
  (params (Key :type Key%20Structure))
  ;[1 1 1] Weapon
  (:Pressed
    (Class|Tank|SetProjectile)))

(event Input|ActionEvents|InputActionweapon_1
  (params (Key :type Key%20Structure))
  ;[1 1 1] Weapon
  (:Pressed
    (Class|Tank|SetProjectile 1)))

(event Input|ActionEvents|InputActionmove_forward
  (params (Key :type Key%20Structure))
  ;[1 1 1] Move
  (:Pressed
    (Class|Tank|MoveForward true))
  (:Released
    (Class|Tank|MoveForward false)))

(event Input|ActionEvents|InputActionmove_backward
  (params (Key :type Key%20Structure))
  ;[1 1 1] Move
  (:Pressed
    (Class|Tank|MoveBackward true))
  (:Released
    (Class|Tank|MoveBackward false)))

(event Input|ActionEvents|InputActionmove_left
  (params (Key :type Key%20Structure))
  ;[1 1 1] Move
  (:Pressed
    (Class|Tank|MoveLeft true))
  (:Released
    (Class|Tank|MoveLeft false)))

(event Input|ActionEvents|InputActionmove_right
  (params (Key :type Key%20Structure))
  ;[1 1 1] Move
  (:Pressed
    (Class|Tank|MoveRight true))
  (:Released
    (Class|Tank|MoveRight false)))

(event Input|AxisEvents|InputAxisaxis_azimuth
  (params (AxisValue :type Float%20%28single-precision%29))
  ;[1 1 1] Axis
  (Transformation|AddLocalRotation (Variables|Default|GetScene) (Math|Rotator|MakeRotator 0.0 0.0 (* AxisValue (Utilities|Time|GetWorldDeltaSeconds) 1e+02)) false false))

(event Input|AxisEvents|InputAxisaxis_altitude
  (params (AxisValue :type Float%20%28single-precision%29))
  ;[1 1 1] Axis
  (Transformation|AddLocalRotation (Variables|Default|GetSpringArm) (Math|Rotator|MakeRotator 0.0 (* AxisValue (Utilities|Time|GetWorldDeltaSeconds) 1e+02) 0.0) false false))

(fn ConstructionScript)