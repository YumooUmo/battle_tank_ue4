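; Player-controlled tank pawn that wires input to its weapon and track-drive components.
; BeginPlay gives StraightWeapon the turret, barrel and two projectile types with ammo, and registers left and right tracks with TrackForceAdapter.
; Move, brake and burst inputs pass through an inputMove graph to the track adapter; weapon inputs call StraightWeapon directly.
; Axis inputs rotate the camera rig; interact detaches the weapon and both drive sides.
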(event EventBeginPlay
  ;[1 1 1] Comment
  (Class|AimingComponent|Setup (Variables|Default|GetStraightWeapon) (Variables|Default|GetTankTurrent) (Variables|Default|GetTankBarrel))
  (Class|StraightWeaponComponent|AddProjectile (Variables|Default|GetStraightWeapon) "/Game/Tank/Projectile/a_projectile.a_projectile_C" 10)
  (Class|StraightWeaponComponent|AddProjectile (Variables|Default|GetStraightWeapon) "/Game/Tank/Projectile/b_projectile.b_projectile_C" 120)
  ;[1 1 1] Comment
  (Class|TrackForceAdapterComponent|SetupLeft (Variables|Default|GetTrackForceAdapter) (Variables|Default|Getleft))
  (Class|TrackForceAdapterComponent|SetupRight (Variables|Default|GetTrackForceAdapter) (Variables|Default|Getright)))

(event Input|ActionEvents|InputActionmove_backward
  (params (Key :type Key%20Structure :default "None"))
  ;[1 1 1] Move
  (:Pressed
    (Utilities|InputMove) ; enters at Backward_true
  )
  (:Released
    (Utilities|InputMove) ; enters at Backward_false
  ))

(event Input|ActionEvents|InputActionmove_forward
  (params (Key :type Key%20Structure :default "None"))
  ;[1 1 1] Move
  (:Pressed
    (Utilities|InputMove :!label _label))
  (:Released
    (goto _label Forward_false)))

(event Input|ActionEvents|InputActionexchange_weapon
  (params (Key :type Key%20Structure :default "None"))
  ;[1 1 1] weapon
  (:Pressed
    (Class|StraightWeaponComponent|ExchangeProjectile (Variables|Default|GetStraightWeapon))))

(event Input|ActionEvents|InputActionaiming
  (params (Key :type Key%20Structure :default "None"))
  (bind _straightweapon (Variables|Default|GetStraightWeapon))
  ;[1 1 1] weapon
  (:Pressed
    (Class|StraightWeaponComponent|Lock _straightweapon true))
  (:Released
    (Class|StraightWeaponComponent|Lock _straightweapon false)))

(event Input|ActionEvents|InputActioninteract
  (params (Key :type Key%20Structure :default "None"))
  (bind _trackforceadapter (Variables|Default|GetTrackForceAdapter))
  (:Pressed
    (Class|AimingComponent|DetachWeapon (Variables|Default|GetStraightWeapon))
    (Class|TrackForceAdapterComponent|DetachLeftDriveside _trackforceadapter)
    (Class|TrackForceAdapterComponent|DetachRightDriveside _trackforceadapter)))

(event Input|ActionEvents|InputActionmove_left
  (params (Key :type Key%20Structure :default "None"))
  ;[1 1 1] Move
  (:Pressed
    (Utilities|InputMove) ; enters at Left_true
  )
  (:Released
    (Utilities|InputMove) ; enters at Left_false
  ))

(event Input|ActionEvents|InputActionmove_right
  (params (Key :type Key%20Structure :default "None"))
  ;[1 1 1] Move
  (:Pressed
    (Utilities|InputMove) ; enters at Right_true
  )
  (:Released
    (Utilities|InputMove) ; enters at Right_false
  ))

(event Input|ActionEvents|InputActionbrake
  (params (Key :type Key%20Structure :default "None"))
  ;[1 1 1] Move
  (:Pressed
    (Utilities|InputMove) ; enters at Brake_true
  )
  (:Released
    (Utilities|InputMove) ; enters at Brake_false
  ))

(event Input|ActionEvents|InputActionburst
  (params (Key :type Key%20Structure :default "None"))
  ;[1 1 1] Move
  (:Pressed
    (Utilities|InputMove) ; enters at Burst_true
  )
  (:Released
    (Utilities|InputMove) ; enters at Burst_false
  ))

(event Input|ActionEvents|InputActionfire
  (params (Key :type Key%20Structure :default "None"))
  ;[1 1 1] weapon
  (:Pressed
    (Class|StraightWeaponComponent|Fire (Variables|Default|GetStraightWeapon))))

(event Input|ActionEvents|InputActionreload
  (params (Key :type Key%20Structure :default "None"))
  ;[1 1 1] weapon
  (:Pressed
    (Class|StraightWeaponComponent|Reload (Variables|Default|GetStraightWeapon))))

(event Input|ActionEvents|InputActionweapon_0
  (params (Key :type Key%20Structure :default "None"))
  ;[1 1 1] weapon
  (:Pressed
    (Class|StraightWeaponComponent|SetProjectile (Variables|Default|GetStraightWeapon))))

(event Input|ActionEvents|InputActionweapon_1
  (params (Key :type Key%20Structure :default "None"))
  ;[1 1 1] weapon
  (:Pressed
    (Class|StraightWeaponComponent|SetProjectile (Variables|Default|GetStraightWeapon) 1)))

(event Input|AxisEvents|InputAxisaxis_altitude
  (params (AxisValue :type Float%20%28single-precision%29))
  ;[1 1 1] Camera
  (Transformation|AddLocalRotation (Variables|Default|GetSpringArm) (Math|Rotator|MakeRotator 0.0 (* AxisValue (Utilities|Time|GetWorldDeltaSeconds) 1e+02) 0.0) false false))

(event Input|AxisEvents|InputAxisaxis_azimuth
  (params (AxisValue :type Float%20%28single-precision%29))
  ;[1 1 1] Camera
  (Transformation|AddLocalRotation (Variables|Default|GetScene) (Math|Rotator|MakeRotator 0.0 0.0 (* AxisValue (Utilities|Time|GetWorldDeltaSeconds) 1e+02)) false false))

(fn ConstructionScript)