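; MyTank_BP is the player-controlled tank Blueprint, wiring its components and input to tank functions.
; On BeginPlay it passes the barrel, turret, both tracks, aiming, weapon and nav movement components to SetUp.
; Input actions call movement, weapon switching, aiming draw, fire, reload and burst functions.
; Look axes rotate the Scene in yaw and the SpringArm in pitch, scaled by delta time, to orbit the camera.
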(event EventBeginPlay
  (Class|Tank|SetUp (Variables|Default|Getbarrel) (Variables|Default|Getturrent) (Variables|Default|Getleft_track) (Variables|Default|Getright_track) (Variables|Default|GetAiming) (Variables|Default|GetWeapon) (Variables|Default|GetForceNavMovement)))

(event Input|ActionEvents|InputActionreload
  (params (Key :type Key%20Structure))
  ;[1 1 1] Weapon
  (:Pressed
    (Class|Tank|Reload)))

(event Input|ActionEvents|InputActionfire
  (params (Key :type Key%20Structure))
  ;[1 1 1] Weapon
  (:Pressed
    (Class|Tank|Fire)))

(event Input|ActionEvents|InputActionburst
  (params (Key :type Key%20Structure))
  ;[1 1 1] Move
  (:Pressed
    (Class|Tank|Burst true))
  (:Released
    (Class|Tank|Burst false)))

(event Input|ActionEvents|InputActionaiming
  (params (Key :type Key%20Structure))
  ;[1 1 1] Aiming
  (:Pressed
    (Class|Tank|Draw true))
  (:Released
    (Class|Tank|Draw false)))

(event Input|ActionEvents|InputActionexchange_weapon
  (params (Key :type Key%20Structure))
  ;[1 1 1] Weapon
  (:Pressed
    (Class|Tank|ExchangeWeapon)))

(event Input|ActionEvents|InputActionweapon_0
  (params (Key :type Key%20Structure))
  ;[1 1 1] Weapon
  (:Pressed
    (Class|Tank|SetWeapon)))

(event Input|ActionEvents|InputActionweapon_1
  (params (Key :type Key%20Structure))
  ;[1 1 1] Weapon
  (:Pressed
    (Class|Tank|SetWeapon 1)))

(event Input|ActionEvents|InputActionmove_forward
  (params (Key :type Key%20Structure))
  ;[1 1 1] Move
  (:Pressed
    (Class|Tank|MoveForward true))
  (:Released
    (Class|Tank|MoveForward false)))

(event Input|ActionEvents|InputActionmove_backward
  (params (Key :type Key%20Structure))
  ;[1 1 1] Move
  (:Pressed
    (Class|Tank|MoveBackward true))
  (:Released
    (Class|Tank|MoveBackward false)))

(event Input|ActionEvents|InputActionmove_left
  (params (Key :type Key%20Structure))
  ;[1 1 1] Move
  (:Pressed
    (Class|Tank|MoveLeft true))
  (:Released
    (Class|Tank|MoveLeft false)))

(event Input|ActionEvents|InputActionmove_right
  (params (Key :type Key%20Structure))
  ;[1 1 1] Move
  (:Pressed
    (Class|Tank|MoveRight true))
  (:Released
    (Class|Tank|MoveRight false)))

(event Input|AxisEvents|InputAxisaxis_azimuth
  (params (AxisValue :type Float%20%28single-precision%29))
  ;[1 1 1] Axis
  (Transformation|AddLocalRotation (Variables|Default|GetScene) (Math|Rotator|MakeRotator 0.0 0.0 (* AxisValue (Utilities|Time|GetWorldDeltaSeconds) 1e+02)) false false))

(event Input|AxisEvents|InputAxisaxis_altitude
  (params (AxisValue :type Float%20%28single-precision%29))
  ;[1 1 1] Axis
  (Transformation|AddLocalRotation (Variables|Default|GetSpringArm) (Math|Rotator|MakeRotator 0.0 (* AxisValue (Utilities|Time|GetWorldDeltaSeconds) 1e+02) 0.0) false false))

(fn ConstructionScript)